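; Base AI enemy character that carries an assault rifle child actor and provides combat, patrol route, movement speed and death functions for its AI controller.
; Attack plays a fire montage whose notify line-traces from the spine, applies rifle damage, then spawns tracer and impact effects or, on a kill, sets the controller passive.
; EquipOrUnequip moves the rifle between sockets by State.
; Die stops AI logic, while StartRagdoll separately enables physics.
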(event `self.ReceiveBeginPlay`
  (bind _asbp_assault_rifle (cast `/Game/ThirdPerson/Blueprints/WeaponBP/weaponChild/BP_AssaultRifle` (`ChildActorComponent.ChildActor` (`self.PrimaryChild`))))
  (set `self.As BP Assault Rifle` _asbp_assault_rifle))

(event `Attack`
  (bind _mesh (`self.Mesh`))
  (bind _returnvalue (`SceneComponent.GetSocketLocation` _mesh "spine_05"))
  (bind _weaponsystem (`/Game/ThirdPerson/Blueprints/WeaponBP/BP_MasterWeapon.WeaponSystem` (`self.As BP Assault Rifle`)))
  (bind _returnvalue_2 (`SceneComponent.GetSocketLocation` (`/Game/ThirdPerson/Blueprints/WeaponBP/BP_MasterWeapon.WeaponMesh` (`self.As BP Assault Rifle`)) "Muzzle"))
  (bind _notifyname (`|PlayMontage` (`self.Mesh`) "/Game/ThirdPerson/Blueprints/Animation/Weapons/Rifle/Montages/MM_Rifle_Fire.MM_Rifle_Fire")
    (:`OnCompleted`
      (`self.OnAttackEnd` :!label _label))
    (:`OnInterrupted`
      (goto _label))
    (:`OnNotifyBegin`
      (switch `name` _notifyname
        (:`Fire`
          (`/Game/ThirdPerson/Blueprints/WeaponBP/weaponChild/BP_AssaultRifle.FireFX_AI` (`self.As BP Assault Rifle`))
          (bind (_outhit _returnvalue_3) (`KismetSystemLibrary.LineTraceSingle` _returnvalue (+ _returnvalue (* (`SceneComponent.GetRightVector` _mesh) (`self.ValidRange`))) "TraceTypeQuery1" false (`|MakeArray` self :!type "Actor Object Reference") "Persistent"))
          (if _returnvalue_3
            ;[0.07177 1 0] Apply hit and damage
            (bind (_killedplayer _validhit) (`/Game/ThirdPerson/Blueprints/WeaponBP/BP_MasterWeapon.ApplyHit` (`self.As BP Assault Rifle`) _outhit))
            ;[0.04688 0.04688 0.04688] Add Hitmarker if we hit another player
            (if _validhit
              (bind _returnvalue_4 (`|CreateWidget` "/Game/ThirdPerson/Blueprints/UI/HitMarker.HitMarker_C"))
              (`UserWidget.AddToViewport` _returnvalue_4 0))
            (if _killedplayer
              ;[1 1 1] Play sound if we got a kill
              (`GameplayStatics.PlaySound2D` "/Game/ThirdPerson/Audio/Sounds/Weapons/kill-sound-effect_Cue.kill-sound-effect_Cue" 1.0 1.0 0.0 null null)
              (bind _asbp_my_aicontroller (cast `/Game/Yuchin/BP/EnemyAI/BP_MyAIController` (`AIBlueprintHelperLibrary.GetAIController` self)))
              (`/Game/Yuchin/BP/EnemyAI/BP_MyAIController.SetStateAsPassive` _asbp_my_aicontroller)
              (else
                (bind (_bblockinghit _binitialoverlap _time _distance _location _impactpoint _normal _impactnormal _physmat _hitactor _hitcomponent _hitbonename _bonename _hititem _elementindex _faceindex _tracestart _traceend) (`GameplayStatics.BreakHitResult` _outhit))
                ;[1 0.2368 0] Calculate bullet tracer and spawn
                (`|SpawnActorFromClass` "/Game/Weapons/BulletTrace/Bullet_Trace.Bullet_Trace_C" (`KismetMathLibrary.MakeTransform` _returnvalue_2 (`KismetMathLibrary.MakeRotFromX` (- (`KismetMathLibrary.SelectVector` _impactpoint _traceend) _returnvalue_2))) "Undefined" "OverrideRootScale" null null)
                ;[0 0.5196 1] Impact VFX
                (`/Game/ThirdPerson/Blueprints/WeaponBP/WeaponSystem.Impact_VFX` _weaponsystem _normal _impactpoint _physmat)
                (`/Game/ThirdPerson/Blueprints/WeaponBP/WeaponSystem.Impact_Decal` _weaponsystem "/Game/Weapons/Decal/Impact_Decal.Impact_Decal_C" _location _impactpoint (0.01 0.02 0.02))))))))))

(event `EquipOrUnequip`
  (bind _mesh (`self.Mesh`))
  (switch `/Game/Yuchin/BP/EnemyAI/Enums/E_AIState` (`self.State`)
    (:`NewEnumerator0`
      (set `self.isEquipping` false)
      (`|PlayMontage` _mesh "/Game/ThirdPerson/Blueprints/Animation/Weapons/Actions/MM_Generic_Unequip1.MM_Generic_Unequip1"
        (:`OnCompleted`
          (`SceneComponent.K2_AttachToComponent` (`self.PrimaryChild`) (`self.Mesh`) "RifleHost_Socket" "SnapToTarget" "SnapToTarget" "SnapToTarget" true))))
    (:`NewEnumerator1`
      (set `self.isEquipping` true)
      (`|PlayMontage` _mesh "/Game/ThirdPerson/Blueprints/Animation/Weapons/Rifle/Montages/MM_Rifle_Equip1.MM_Rifle_Equip1"
        (:`then`
          (`SceneComponent.K2_AttachToComponent` (`self.PrimaryChild`) (`self.Mesh`) "Rifle_Socket" "SnapToTarget" "SnapToTarget" "SnapToTarget" true :!label _label_2))
        (:`OnCompleted`
          (goto _label_2))
        (:`OnInterrupted`
          _))
      (`self.OnEquipEnd`))))

(fn `Die`
  (if (not (`self.bEnemyDead`))
    (set `self.bEnemyDead` true)
    (`BrainComponent.StopLogic` (`AIController.BrainComponent` (`AIBlueprintHelperLibrary.GetAIController` self)) "")))

(fn `GetPatrolRoute`
  (returns (PatrolRoute :type "/Game/Yuchin/BP/EnemyAI/BP_EnemyPatrolRoute Object Reference"))
  (return (`self.PatrolRoute`)))

(fn `SetMovementSpeed`
  (params (Speed :type "/Game/Yuchin/BP/EnemyAI/Enums/E_MovementSpeed Enum" :default "NewEnumerator0"))
  (returns (SpeedValue :type "Float (double-precision)"))
  (bind _output_get (set `CharacterMovementComponent.MaxWalkSpeed` (select `/Game/Yuchin/BP/EnemyAI/Enums/E_MovementSpeed` Speed :`NewEnumerator1` 250.0 :`NewEnumerator2` 300.0 :`NewEnumerator3` 500.0 :!type "Float (single-precision)") (`self.CharacterMovement`)))
  (return _output_get))

(fn `StartRagdoll`
  (`|ExecutionSequence`
    (:`then_0`
      ;[0.04688 0.04688 0.04688] Disable Character Movement
      (`CharacterMovementComponent.DisableMovement` (`self.CharacterMovement`)))
    (:`then_1`
      ;[0 1 0.4178] Disable Capsule Component Collision
      (`PrimitiveComponent.SetCollisionEnabled` (`self.CapsuleComponent`) "NoCollision"))
    (:`then_2`
      ;[0 0.5502 1] Enable Ragdoll Physics on body mesh
      (`PrimitiveComponent.SetSimulatePhysics` (`self.Mesh`) true))
    (:`then_3`
      ;[1 0 0.03409] Hide Weapons
      (`SceneComponent.SetVisibility` (`self.PrimaryChild`) false true))))

(fn `UserConstructionScript`)