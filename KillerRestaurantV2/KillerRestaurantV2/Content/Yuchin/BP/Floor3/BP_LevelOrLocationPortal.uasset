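; BP_LevelOrLocationPortal is an interactable portal that moves the player to another level or another spot in the same level.
; Its sphere overlap registers it as the third-person character's current overlapped item and shows an interaction widget labelled with the WhereToMove destination.
; MoveToLevelOrLoc checks the MoveToLevel flag, then looks up WhereToMove in a map to open a level or teleport the player, printing a message when no entry exists.
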(event `self.ReceiveBeginPlay`
  (`SceneComponent.SetVisibility` (`self.Widget`) false false)
  (bind _asw_environment_interaction (cast `/Game/ThirdPerson/Blueprints/Interaction/DemoUI/W_EnvironmentInteraction` (`WidgetComponent.GetWidget` (`self.Widget`))))
  (set `self.As W Environment Interaction` _asw_environment_interaction))

(event `self.Sphere.OnComponentBeginOverlap`
  (params (OverlappedComponent :type "PrimitiveComponent Object Reference") (OtherActor :type "Actor Object Reference") (OtherComp :type "PrimitiveComponent Object Reference") (OtherBodyIndex :type Integer) (bFromSweep :type Boolean) (SweepResult :type "HitResult Structure (by ref)"))
  (bind _asbp_third_person_character (cast `/Game/ThirdPerson/Blueprints/BP_ThirdPersonCharacter` OtherActor))
  (set `/Game/ThirdPerson/Blueprints/BP_ThirdPersonCharacter.CurrentOverlappedItem` self _asbp_third_person_character)
  (`/Game/ThirdPerson/Blueprints/Interaction/DemoUI/W_EnvironmentInteraction.SetInteractionText` (`self.As W Environment Interaction`) (`self.WhereToMove`))
  (`SceneComponent.SetVisibility` (`self.Widget`) true false))

(event `self.Sphere.OnComponentEndOverlap`
  (params (OverlappedComponent :type "PrimitiveComponent Object Reference") (OtherActor :type "Actor Object Reference") (OtherComp :type "PrimitiveComponent Object Reference") (OtherBodyIndex :type Integer))
  (bind _asbp_third_person_character (cast `/Game/ThirdPerson/Blueprints/BP_ThirdPersonCharacter` OtherActor))
  (set `/Game/ThirdPerson/Blueprints/BP_ThirdPersonCharacter.CurrentOverlappedItem` null _asbp_third_person_character)
  (`SceneComponent.SetVisibility` (`self.Widget`) false false))

(event `MoveToLevelOrLoc`
  (params (Player :type "/Game/ThirdPerson/Blueprints/BP_ThirdPersonCharacter Object Reference"))
  (bind (_value _returnvalue) (`BlueprintMapLibrary.Map_Find` (`self.PortalDestinationMap`) (`self.WhereToMove`)))
  (bind (_value_2 _returnvalue_2) (`BlueprintMapLibrary.Map_Find` (`self.WhereToMoveLevelMaps`) (`self.WhereToMove`)))
  (if (`self.bMoveToLevel`)
    (if _returnvalue_2
      (`GameplayStatics.OpenLevel` _value_2) ; 다른 레벨 이동
      (else
        (`KismetSystemLibrary.PrintString` "Don't have level name in map")))
    (elif _returnvalue
      (`self.K2_TeleportTo` :`self` Player :`DestLocation` _value) ; 같은 레벨에서 위치만 이동
      (else
        (`KismetSystemLibrary.PrintString` "Don't have location in map")))))

(fn `UserConstructionScript`)