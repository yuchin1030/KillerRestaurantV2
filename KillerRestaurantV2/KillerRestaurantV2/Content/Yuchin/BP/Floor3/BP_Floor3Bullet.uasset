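; BP_Floor3Bullet is an ammo item for Floor 3 that shows either rifle or pistol ammo.
; Its construction script runs the parent's, then switches on the item name in Floor3ItemData to set the matching static mesh.
; The event graph holds only disabled default events, so the Blueprint adds no runtime logic of its own.
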(fn `UserConstructionScript`
  (`parent.UserConstructionScript`)
  (switch `name` (`.ItemName_4_E494307244C7AD7297604BBDAF9ACEE9` (break `/Game/Yuchin/BP/Floor3/Floor3ItemData` (`self.Floor3_ItemData`)))
    (:`Rifle Ammo`
      (`StaticMeshComponent.SetStaticMesh` (`self.StaticMesh`) "/Game/Yuchin/Assets/ammo-boxes-toon-style/SM_RifleAmmo.SM_RifleAmmo"))
    (:`Pistol Ammo`
      (`StaticMeshComponent.SetStaticMesh` (`self.StaticMesh`) "/Game/Yuchin/Assets/ammo-boxes-toon-style/SM_PistolAmmo.SM_PistolAmmo"))))