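; Base pickup actor for Floor 3 items that floats in place and shows an interaction prompt when the player is nearby.
; BeginPlay spawns a Niagara effect (NS_Flour), hides the widget component and caches its W_EnvironmentInteraction.
; Tick bobs the actor vertically by adding a sine offset each frame.
; Sphere overlaps set or clear CurrentOverlappedItem on BP_ThirdPersonCharacter and toggle the prompt, labelled with the item data's name.
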(event `self.ReceiveBeginPlay`
  (`NiagaraFunctionLibrary.SpawnSystemAtLocation` "/Game/Generic_Item_Destruction_FX/Visual_Effects/NiagaraSystem/NS_Flour.NS_Flour" (`self.K2_GetActorLocation`))
  (`SceneComponent.SetVisibility` (`self.Widget`) false false)
  (bind _asw_environment_interaction (cast `/Game/ThirdPerson/Blueprints/Interaction/DemoUI/W_EnvironmentInteraction` (`WidgetComponent.GetWidget` (`self.Widget`))))
  (set `self.As W Environment Interaction` _asw_environment_interaction))

(event `self.ReceiveTick`
  (params (DeltaSeconds :type "Float (single-precision)"))
  (bind _output_get (set `self.time` (+ (`self.time`) DeltaSeconds)))
  (`self.K2_SetActorLocation` (+ (`self.K2_GetActorLocation`) (`KismetMathLibrary.MakeVector` 0.0 0.0 (* (`KismetMathLibrary.Sin` (* _output_get 3.0)) 0.2)))))

(event `self.Sphere.OnComponentBeginOverlap`
  (params (OverlappedComponent :type "PrimitiveComponent Object Reference") (OtherActor :type "Actor Object Reference") (OtherComp :type "PrimitiveComponent Object Reference") (OtherBodyIndex :type Integer) (bFromSweep :type Boolean) (SweepResult :type "HitResult Structure (by ref)"))
  (bind _asbp_third_person_character (cast `/Game/ThirdPerson/Blueprints/BP_ThirdPersonCharacter` OtherActor))
  (set `/Game/ThirdPerson/Blueprints/BP_ThirdPersonCharacter.CurrentOverlappedItem` self _asbp_third_person_character)
  (`/Game/ThirdPerson/Blueprints/Interaction/DemoUI/W_EnvironmentInteraction.SetInteractionText` (`self.As W Environment Interaction`) (`KismetStringLibrary.Conv_NameToString` (`.ItemName_4_E494307244C7AD7297604BBDAF9ACEE9` (break `/Game/Yuchin/BP/Floor3/Floor3ItemData` (`self.Floor3_ItemData`)))))
  (`SceneComponent.SetVisibility` (`self.Widget`) true false))

(event `self.Sphere.OnComponentEndOverlap`
  (params (OverlappedComponent :type "PrimitiveComponent Object Reference") (OtherActor :type "Actor Object Reference") (OtherComp :type "PrimitiveComponent Object Reference") (OtherBodyIndex :type Integer))
  (bind _asbp_third_person_character (cast `/Game/ThirdPerson/Blueprints/BP_ThirdPersonCharacter` OtherActor))
  (set `/Game/ThirdPerson/Blueprints/BP_ThirdPersonCharacter.CurrentOverlappedItem` null _asbp_third_person_character)
  (`SceneComponent.SetVisibility` (`self.Widget`) false false))

(fn `UserConstructionScript`)