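; BP_ItemSpawner is a breakable actor that can drop an item when destroyed.
; Each ItemSpawnerOnHit call plays the NS_Wood2 effect at its location and deducts a fixed amount from Health while it is above zero.
; A hit received with Health already depleted spawns a new actor of SpawnItem's class at the spawner's transform, if that reference is valid, then destroys the spawner.
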(event `ItemSpawnerOnHit`
  (`NiagaraFunctionLibrary.SpawnSystemAtLocation` "/Game/Generic_Item_Destruction_FX/Visual_Effects/NiagaraSystem/NS_Wood2.NS_Wood2" (`self.K2_GetActorLocation`))
  (if (> (`self.Health`) 0.0)
    (set `self.Health` (- (`self.Health`) 30.0))
    (else
      (bind _spawnitem (`self.SpawnItem`)
        (:`then`
          (`|SpawnActorFromClass` (`GameplayStatics.GetObjectClass` _spawnitem) (`self.GetTransform`) "Undefined" "MultiplyWithRoot" null null))
        (:`else`
          _))
      (`self.K2_DestroyActor`))))

(fn `UserConstructionScript`)