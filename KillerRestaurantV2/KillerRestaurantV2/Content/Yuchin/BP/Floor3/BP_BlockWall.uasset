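; A blocking wall on Floor 3 that names the item it requires and can fade away to open.
; While the third-person character overlaps its box, it registers as that character's current overlapped item and shows a widget with the required item name.
; The CanOpenWall event, which does no item check itself, runs a timeline driving the material's opacity fade parameter, then destroys the actor.
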(event `self.ReceiveBeginPlay`
  (`SceneComponent.SetVisibility` (`self.Widget`) false false))

(event `self.boxColl.OnComponentBeginOverlap`
  (params (OverlappedComponent :type "PrimitiveComponent Object Reference") (OtherActor :type "Actor Object Reference") (OtherComp :type "PrimitiveComponent Object Reference") (OtherBodyIndex :type Integer) (bFromSweep :type Boolean) (SweepResult :type "HitResult Structure (by ref)"))
  (bind _asbp_third_person_character (cast `/Game/ThirdPerson/Blueprints/BP_ThirdPersonCharacter` OtherActor))
  (set `/Game/ThirdPerson/Blueprints/BP_ThirdPersonCharacter.CurrentOverlappedItem` self _asbp_third_person_character)
  (bind _aswbp_block_wall_required_item (cast `/Game/Yuchin/UI/WBP_BlockWallRequiredItem` (`WidgetComponent.GetWidget` (`self.Widget`))))
  (`/Game/Yuchin/UI/WBP_BlockWallRequiredItem.ShowRequiredItem` _aswbp_block_wall_required_item (`self.requiredItemName`))
  (`SceneComponent.SetVisibility` (`self.Widget`) true false))

(event `self.boxColl.OnComponentEndOverlap`
  (params (OverlappedComponent :type "PrimitiveComponent Object Reference") (OtherActor :type "Actor Object Reference") (OtherComp :type "PrimitiveComponent Object Reference") (OtherBodyIndex :type Integer))
  (bind _asbp_third_person_character (cast `/Game/ThirdPerson/Blueprints/BP_ThirdPersonCharacter` OtherActor))
  (set `/Game/ThirdPerson/Blueprints/BP_ThirdPersonCharacter.CurrentOverlappedItem` null _asbp_third_person_character)
  (`SceneComponent.SetVisibility` (`self.Widget`) false false))

(event `CanOpenWall`
  (bind (_direction _newtrack_0) (`Timeline|Timeline`)
    (:`Update`
      (`MeshComponent.SetScalarParameterValueOnMaterials` (`self.smComp`) "OpacityFadeAlpha" _newtrack_0))
    (:`Finished`
      (`self.K2_DestroyActor`))))

(fn `UserConstructionScript`)