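; Horizontal billboard cosmetic for CyberTown that shows custom, glowing text on both its front and back.
; The construction script extends the parent's, applying font, size and text to two text renders and offsetting them, with horizontal shift mirrored on the back.
; Both renders share a dynamic instance of MM_Billboard_Text, which receives emissive color, intensity and wave settings.
; All setup happens at construction, as the event graph holds only disabled stubs.
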(fn `UserConstructionScript`
  (locals (savedTRFrontTransform :type "Transform Structure") (savedTRBackTransform :type "Transform Structure"))
  (bind _savedtrfronttransform (`local.savedTRFrontTransform`))
  (bind (_textoffset_x _textoffset_y) (`KismetMathLibrary.BreakVector2D` (`self.TextOffset`)))
  (bind _savedtrbacktransform (`local.savedTRBackTransform`))
  (bind (_textoffset_x_2 _textoffset_y_2) (`KismetMathLibrary.BreakVector2D` (`self.TextOffset`)))
  (`parent.UserConstructionScript`)
  ;[1 1 1] Text General Settings
  (`TextRenderComponent.SetFont` (`self.TextRender-Front`) (`self.TextFont`))
  (`TextRenderComponent.SetFont` (`self.TextRender-Back`) (`self.TextFont`))
  (`TextRenderComponent.SetWorldSize` (`self.TextRender-Front`) (`self.FontSize`))
  (`TextRenderComponent.SetWorldSize` (`self.TextRender-Back`) (`self.FontSize`))
  (`TextRenderComponent.K2_SetText` (`self.TextRender-Back`) (`self.Text`))
  (`TextRenderComponent.K2_SetText` (`self.TextRender-Front`) (`self.Text`))
  (set `local.savedTRFrontTransform` (`SceneComponent.GetRelativeTransform` (`self.TextRender-Front`)))
  (set `local.savedTRBackTransform` (`SceneComponent.GetRelativeTransform` (`self.TextRender-Back`)))
  (`SceneComponent.K2_SetRelativeLocation` (`self.TextRender-Front`) (`KismetMathLibrary.MakeVector` (.x (.location _savedtrfronttransform)) (- (.y (.location _savedtrfronttransform)) _textoffset_x) (+ (.z (.location _savedtrfronttransform)) _textoffset_y)) false false)
  (`SceneComponent.K2_SetRelativeLocation` (`self.TextRender-Back`) (`KismetMathLibrary.MakeVector` (.x (.location _savedtrbacktransform)) (+ _textoffset_x_2 (.y (.location _savedtrbacktransform))) (+ (.z (.location _savedtrbacktransform)) _textoffset_y_2)) false false)
  (bind _returnvalue (`KismetMaterialLibrary.CreateDynamicMaterialInstance` "/Game/CyberTown/Blueprints/Cosmetic/Billboard/Material/MM_Billboard_Text.MM_Billboard_Text"))
  (bind _output_get (set `self.DynamicMaterialInstance_Text` _returnvalue))
  (`PrimitiveComponent.SetMaterial` (`self.TextRender-Front`) 0 _output_get)
  (`PrimitiveComponent.SetMaterial` (`self.TextRender-Back`) 0 _output_get)
  (`MaterialInstanceDynamic.SetVectorParameterValue` (`self.DynamicMaterialInstance_Text`) "Emissive_Color" (`self.TextEmissiveColor`))
  (`MaterialInstanceDynamic.SetScalarParameterValue` (`self.DynamicMaterialInstance_Text`) "Emissive_Intensity" (`self.EmissiveIntensity`))
  (`MaterialInstanceDynamic.SetScalarParameterValue` (`self.DynamicMaterialInstance_Text`) "bWave" (`KismetMathLibrary.Conv_BoolToDouble` (`self.RandomWave?`)))
  (`MaterialInstanceDynamic.SetVectorParameterValue` (`self.DynamicMaterialInstance_Text`) "Wave_Speed" (make `LinearColor` 0.0 (`self.WaveSpeed`) 0.0 1.0)))