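; BP_Neon_Obro is a cosmetic neon prop for CyberTown with a configurable texture, emissive color, opacity and motion speed.
; The construction script creates a dynamic instance of M_Neon_Obro, assigns it to the ObroSM mesh and writes the actor's variables into its parameters.
; The X and Y rotation speeds are packed into one Speed vector, leaving any animation to the material, as the event graph holds no active logic.
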(fn `UserConstructionScript`
  (bind _returnvalue (`PrimitiveComponent.CreateDynamicMaterialInstance` (`self.Obro_SM`) 0 "/Game/CyberTown/Blueprints/Cosmetic/NeonObro/Material/M_Neon_Obro.M_Neon_Obro" "None"))
  (bind _output_get (set `self.DynamicMaterialInstance` _returnvalue))
  (`MaterialInstanceDynamic.SetScalarParameterValue` _returnvalue "Opacity" (`self.Opacity`))
  (`MaterialInstanceDynamic.SetScalarParameterValue` _output_get "Opacity" (`self.Opacity`))
  (`PrimitiveComponent.SetMaterial` (`self.Obro_SM`) 0 (`self.DynamicMaterialInstance`))
  (`MaterialInstanceDynamic.SetTextureParameterValue` (`self.DynamicMaterialInstance`) "MainTexture" (`self.MainTexture`))
  (`MaterialInstanceDynamic.SetVectorParameterValue` (`self.DynamicMaterialInstance`) "Speed" (`KismetMathLibrary.MakeColor` (`self.RotationSpeedX`) (`self.RotationSpeedY`)))
  (`MaterialInstanceDynamic.SetVectorParameterValue` (`self.DynamicMaterialInstance`) "EmissiveColor" (`self.EmissiveColor`)))