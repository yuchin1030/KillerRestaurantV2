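; Cosmetic hover car for CyberTown that repeatedly makes a passing movement.
; On BeginPlay it runs the parent logic, then starts a timeline whose movement track sets the relative location of its Parent component, without sweeping.
; When the timeline finishes, it pauses briefly and replays from the start, looping the pass indefinitely without using Tick.
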(event `self.ReceiveBeginPlay`
  (`parent.ReceiveBeginPlay`)
  (bind (_direction _movementtrack) (`Timeline|Move_Timeline` :!label _label)
    (:`Update`
      (`SceneComponent.K2_SetRelativeLocation` (`self.Parent`) _movementtrack false false))
    (:`Finished`
      (`KismetSystemLibrary.Delay` 1.0)
      (goto _label :!via `PlayFromStart`))))

(fn `UserConstructionScript`
  (`parent.UserConstructionScript`))