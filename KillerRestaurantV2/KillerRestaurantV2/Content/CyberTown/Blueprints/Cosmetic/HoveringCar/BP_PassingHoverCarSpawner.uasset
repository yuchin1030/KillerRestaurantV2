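; Cosmetic spawner that creates a stream of BP_HoverCar_Passing cars as passing hover-car traffic.
; On BeginPlay it runs an unrolled chain of five spawns separated by SpawnDelay, with no loop or repeat.
; Each car takes its location from the Sphere component and its rotation from MovingDirection.
; According to the graph comment, the cars move forward and reset their position at a certain point.
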(event `self.ReceiveBeginPlay`
  (bind _returnvalue (`KismetMathLibrary.MakeTransform` (`SceneComponent.K2_GetComponentLocation` (`self.Sphere`)) (`SceneComponent.K2_GetComponentRotation` (`self.MovingDirection`))))
  ;[1 1 1] Spawns multiple hover cars of type "Passing". These spawned cars will move forward and reset their position when reach a certain point.
  (`|SpawnActorFromClass` "/Game/CyberTown/Blueprints/Cosmetic/HoveringCar/BP_HoverCar_Passing.BP_HoverCar_Passing_C" _returnvalue "Undefined" "OverrideRootScale" null null)
  (`KismetSystemLibrary.Delay` (`self.SpawnDelay`))
  (`|SpawnActorFromClass` "/Game/CyberTown/Blueprints/Cosmetic/HoveringCar/BP_HoverCar_Passing.BP_HoverCar_Passing_C" _returnvalue "Undefined" "OverrideRootScale" null null)
  (`KismetSystemLibrary.Delay` (`self.SpawnDelay`))
  (`|SpawnActorFromClass` "/Game/CyberTown/Blueprints/Cosmetic/HoveringCar/BP_HoverCar_Passing.BP_HoverCar_Passing_C" _returnvalue "Undefined" "OverrideRootScale" null null)
  (`KismetSystemLibrary.Delay` (`self.SpawnDelay`))
  (`|SpawnActorFromClass` "/Game/CyberTown/Blueprints/Cosmetic/HoveringCar/BP_HoverCar_Passing.BP_HoverCar_Passing_C" _returnvalue "Undefined" "OverrideRootScale" null null)
  (`KismetSystemLibrary.Delay` (`self.SpawnDelay`))
  (`|SpawnActorFromClass` "/Game/CyberTown/Blueprints/Cosmetic/HoveringCar/BP_HoverCar_Passing.BP_HoverCar_Passing_C" _returnvalue "Undefined" "OverrideRootScale" null null)
  (`KismetSystemLibrary.Delay` (`self.SpawnDelay`)))

(fn `UserConstructionScript`)