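; BP_HoverCar is a cosmetic hovering car for CyberTown that bobs and rolls when its engine is flagged as running.
; On BeginPlay a timeline drives the parent component's height and roll, with an adjustable play rate.
; The construction script sets steam particle auto-activation from the engine flag and toggles four light-volume emissions.
; It registers the car mesh's body and emissive colors with the parent class's material customization system.
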(event `self.ReceiveBeginPlay`
  (if (`self.isEngineRunning?`)
    (bind (_direction _rot _up_down) (`Timeline|Hover_Timeline` :!via `PlayFromStart`)
      (:`Update`
        (`SceneComponent.K2_SetRelativeLocationAndRotation` (`self.Parent`) _up_down (`KismetMathLibrary.MakeRotator` _rot) false false)
        (`TimelineComponent.SetPlayRate` (`self.Hover_Timeline`) (`self.HoveringPlayrate`))))))

(fn `ChildMaterialVariablesSetup`
  (`KismetArrayLibrary.Array_Add` (`self.MaterialCustomizations`) (make `/Game/CyberTown/Blueprints/Cosmetic/CustomzableAsset/CustomizableParent/S_MaterialCustomization` (`self.SM_Car_01a`) (`|MakeArray` (make `/Game/CyberTown/Blueprints/Cosmetic/CustomzableAsset/CustomizableParent/S_MaterialIndex` 0 (make `/Game/CyberTown/Blueprints/Cosmetic/CustomzableAsset/CustomizableParent/S_MaterialParameterOptions` false "" "Main_AlbedoTint" true "BodyColor1" "Main_TintColor_1" true "BodyColor2" "Main_TintColor_2" true "EmissiveColor")))))
  (`parent.ChildMaterialVariablesSetup`))

(fn `ColorSetup`)

(fn `EngineRunningSetup`
  ;[1 1 1] Setup child components (Sound, Particle Systems) for Engine Running Option
  (for _array_element (`SceneComponent.GetChildrenComponents` (`self.SteamParticles`) true)
    (bind _asparticle_system_component (cast `ParticleSystemComponent` _array_element))
    (`ActorComponent.SetAutoActivate` _asparticle_system_component (`self.isEngineRunning?`))))

(fn `UserConstructionScript`
  (`parent.UserConstructionScript`)
  (`self.EngineRunningSetup`)
  (`SceneComponent.SetVisibility` (`self.LightVolumeEmission1`) (`self.haveLightVolumeEmission`) false)
  (`SceneComponent.SetVisibility` (`self.LightVolumeEmission2`) (`self.haveLightVolumeEmission`) false)
  (`SceneComponent.SetVisibility` (`self.LightVolumeEmission3`) (`self.haveLightVolumeEmission`) false)
  (`SceneComponent.SetVisibility` (`self.LightVollumeEmission4`) (`self.haveLightVolumeEmission`) false))