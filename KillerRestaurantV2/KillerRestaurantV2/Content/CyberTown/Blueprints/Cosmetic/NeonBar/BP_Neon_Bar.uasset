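; BP_Neon_Bar is a cosmetic neon bar prop with configurable glow and an optional point light.
; Its construction script creates a dynamic material instance from MasterMaterial on the neon mesh and applies emissive color and intensity.
; AddLight toggles the PointLight, making it visible and Static when on, or hidden and Movable when off.
; When the light is on, SetColorSameAsEmissive can match its color to the emissive color.
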(fn `UserConstructionScript`
  (locals (neon :type "PrimitiveComponent Object Reference") (Local_lightLocation :type "Vector Structure") (Local_billboardHeight :type "Float (double-precision)"))
  (bind _pointlight (`self.PointLight`))
  (bind _dynamicmaterialinstance (`self.DynamicMaterialInstance`))
  (bind _output_get (set `local.neon` (`self.SM_Neon_01a`)))
  (`/Engine/EditorBlueprintResources/StandardMacros.IsValid` _output_get
    (:`Is Valid`
      (`|ExecutionSequence`
        (:`then_0`
          (bind _returnvalue (`PrimitiveComponent.CreateDynamicMaterialInstance` (`local.neon`) 0 (`self.MasterMaterial`) "None"))
          (set `self.DynamicMaterialInstance` _returnvalue)
          (`PrimitiveComponent.SetMaterial` (`local.neon`) 0 (`self.DynamicMaterialInstance`))
          (`MaterialInstanceDynamic.SetVectorParameterValue` _dynamicmaterialinstance "Emissive_Color" (`self.EmissiveColor`))
          (`MaterialInstanceDynamic.SetScalarParameterValue` _dynamicmaterialinstance "Emissive_Intensity" (`self.EmissiveIntensity`)))
        (:`then_1`
          (if (`self.bAddLight`)
            (`SceneComponent.SetVisibility` _pointlight true true)
            (`SceneComponent.SetMobility` _pointlight "Static")
            (`SceneComponent.SetHiddenInGame` _pointlight false true)
            (if (`self.bSetColorSameAsEmissive`)
              (`LightComponent.SetLightColor` (`self.PointLight`) (`self.EmissiveColor`) true))
            (else
              (`SceneComponent.SetVisibility` _pointlight false true)
              (`SceneComponent.SetMobility` _pointlight "Movable")
              (`SceneComponent.SetHiddenInGame` _pointlight true true))))))))