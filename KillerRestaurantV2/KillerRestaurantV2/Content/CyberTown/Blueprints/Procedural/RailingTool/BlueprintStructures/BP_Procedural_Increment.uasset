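; Procedural railing tool Blueprint that lays static meshes along a spline as deformed spline mesh segments, built in the Construction Script.
; The first mesh's X size sets segment length and, with spline length, the segment count.
; Each segment gets clamped distances and length-normalized tangents, cycles through the mesh array in order, and applies configurable collision.
; Segments shorter than a threshold fraction of full length receive no mesh.
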(fn `GenerateProceduralMesh`
  (locals (SegmentIndex :type Integer) (MeshIndex :type Integer) (SelectedMesh :type "StaticMesh Object Reference") (GeneratedMeshComponent :type "SplineMeshComponent Object Reference") (StartPos :type "Vector Structure") (EndPos :type "Vector Structure") (StartTan :type "Vector Structure") (EndTan :type "Vector Structure") (StartDis :type "Float (double-precision)") (EndDis :type "Float (double-precision)"))
  (bind _segmentlength (`self.SegmentLength`))
  (bind _segmentlength_2 (`self.SegmentLength`))
  (bind _output (`|GetArrayItem` (`self.SelectionMeshes`)))
  (bind _sizevector_x (`KismetMathLibrary.BreakVector` (`self.GetCorrectSizeForSegment` _output)))
  (`/Engine/EditorBlueprintResources/StandardMacros.IsValid` _output
    (:`Is Valid`
      ;[1 1 1] Segment Length And Count Calculations
      (set `self.SegmentLength` _sizevector_x)
      (bind _output_get (set `self.SectionCountMax` (`.ReturnValue` (`KismetMathLibrary.FMod` (`SplineComponent.GetSplineLength` (`self.MainSpline`)) (`self.SegmentLength`)))))
      (for _index (range (+ _output_get 1))
        (set `local.SegmentIndex` _index)
        ;[1 1 1] Comment
        (set `local.SelectedMesh` (`|GetArrayItem` (`self.SelectionMeshes`) (`local.MeshIndex`)))
        (bind _returnvalue (`AddComponent|NODE_AddSplineMeshComponent-0` :`RelativeTransform` (`KismetMathLibrary.MakeTransform` (0.0 0.0 0.0) (struct) (`self.Scaler`))))
        (bind _output_get_2 (set `local.GeneratedMeshComponent` _returnvalue))
        (`KismetArrayLibrary.Array_Add` (`self.splineMeshComponents`) _output_get_2)
        ;[1 1 1] Start and End Distance
        (set `local.StartDis` (`KismetMathLibrary.FClamp` (* (`local.SegmentIndex`) (`self.SegmentLength`)) 0.0 (`self.SplineEndPointDistance`)))
        (set `local.EndDis` (`KismetMathLibrary.FClamp` (* (+ (`local.SegmentIndex`) 1) (`self.SegmentLength`)) 0.0 (`self.SplineEndPointDistance`)))
        ;[1 1 1] Generate mesh or not?
        (if (>= (- (`local.EndDis`) (`local.StartDis`)) (* (`self.SegmentLength`) (`self.OffsetBeforeAttachMesh`)))
          ;[1 1 1] Start and End Pos
          (set `local.StartPos` (`SplineComponent.GetLocationAtDistanceAlongSpline` (`self.MainSpline`) (`local.StartDis`) "Local"))
          (set `local.EndPos` (`SplineComponent.GetLocationAtDistanceAlongSpline` (`self.MainSpline`) (`local.EndDis`) "Local"))
          ;[1 1 1] Start and End Tangent
          (set `local.StartTan` (`KismetMathLibrary.ClampVectorSize` (`SplineComponent.GetTangentAtDistanceAlongSpline` (`self.MainSpline`) (`local.StartDis`) "Local") _segmentlength_2 _segmentlength_2))
          (set `local.EndTan` (`KismetMathLibrary.ClampVectorSize` (`SplineComponent.GetTangentAtDistanceAlongSpline` (`self.MainSpline`) (`local.EndDis`) "Local") _segmentlength _segmentlength))
          (`StaticMeshComponent.SetStaticMesh` (`local.GeneratedMeshComponent`) (`local.SelectedMesh`))
          (`SplineMeshComponent.SetStartAndEnd` (`local.GeneratedMeshComponent`) (`local.StartPos`) (`local.StartTan`) (`local.EndPos`) (`local.EndTan`) false)
          (`SplineMeshComponent.SetForwardAxis` (`local.GeneratedMeshComponent`) "X" true)
          (`PrimitiveComponent.SetCollisionEnabled` (`local.GeneratedMeshComponent`) (`self.CollisionEnable`))
          (`PrimitiveComponent.SetCollisionObjectType` (`local.GeneratedMeshComponent`) (`self.CollisionType`))
          (bind _result (`/Engine/EditorBlueprintResources/StandardMacros.IncrementInt` (`local.MeshIndex`))
            (:`  `
              (if (> _result (- (`KismetArrayLibrary.Array_Length` (`self.SelectionMeshes`)) 1))
                (set `local.MeshIndex` 0)))))))))

(fn `UserConstructionScript`
  (`parent.UserConstructionScript`)
  (`self.GenerateProceduralMesh`))