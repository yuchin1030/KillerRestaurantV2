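; BP_ProceduralParent is a parent Blueprint for procedural spline-based structures in the railing tool.
; Its construction script clears the spline mesh component list, caches the spline's end distance, forces actor scale to one and applies the Scaler to the main spline instead.
; Helper functions measure a static mesh's bounding-box extents per axis and convert a percentage into a scale multiplier for segments.
; The event graph holds no active logic.
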(fn `GetCorrectSizeForSegment`
  (params (StaticMesh :type "StaticMesh Object Reference"))
  (returns (SizeVector :type "Vector Structure"))
  (bind _returnvalue (`StaticMesh.GetBoundingBox` StaticMesh))
  (return (`KismetMathLibrary.MakeVector` (+ (`KismetMathLibrary.Abs` (.x (`.Max` (break `Box` _returnvalue)))) (`KismetMathLibrary.Abs` (.x (break `Box` _returnvalue)))) (+ (`KismetMathLibrary.Abs` (.y (break `Box` _returnvalue))) (`KismetMathLibrary.Abs` (.y (`.Max` (break `Box` _returnvalue))))) (+ (`KismetMathLibrary.Abs` (.z (`.Max` (break `Box` _returnvalue)))) (`KismetMathLibrary.Abs` (.z (break `Box` _returnvalue)))))))

(fn `GetScaleFromPercentage`
  (params (Percentage :type "Float (double-precision)"))
  (returns (Scale :type "Float (double-precision)"))
  (return (+ (/ Percentage 100.0) 1.0)))

(fn `UserConstructionScript`
  (bind _mainspline (`self.MainSpline`))
  (`KismetArrayLibrary.Array_Clear` (`self.splineMeshComponents`))
  (set `self.SplineEndPointDistance` (`SplineComponent.GetDistanceAlongSplineAtSplinePoint` _mainspline (- (`SplineComponent.GetNumberOfSplinePoints` _mainspline) 1)))
  (`self.SetActorScale3D` (1.0 1.0 1.0))
  (`SceneComponent.SetRelativeScale3D` (`self.MainSpline`) (`self.Scaler`)))