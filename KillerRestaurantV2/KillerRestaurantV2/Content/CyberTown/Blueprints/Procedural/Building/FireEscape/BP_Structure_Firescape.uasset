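; Procedural fire escape structure that stacks optional starting and ending pieces around repeated middle sections, with total count clamped in construction.
; Generate spawns each piece from a template, offsets it by height accumulated from bounding boxes, then generates its additional parts.
; The ending piece flips 180 degrees based on the last middle index's parity.
; ManageOptions resizes the ladder transforms to the ladder count and registers up to three optional ladder mesh slots.
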(fn `Generate`
  (locals (Local_currentStructureIndex :type Integer) (Local_currentCreatedTemplateActor :type "ChildActorComponent Object Reference") (Local_currentAssociateMeshes :type "Map of String to ChildActorComponent Object Reference") (Local_middleFirescapeCount :type Integer) (Local_isEvenIndex :type Boolean) (Local_endFirescapePieceRotation :type "Rotator Structure"))
  (bind _local_currentcreatedtemplateactor (`local.Local_currentCreatedTemplateActor`))
  (`|ExecutionSequence`
    (:`then_0`
      (if (`self.AddStartingPiece?`)
        (bind _createdtemplate (`self.CreateNewTemplate` (`self.FirescapeStartingActor`)))
        (bind (_parentactor _associativechildactor) (break `/Game/CyberTown/Blueprints/Procedural/Building/BlueprintStructures/S_CreatedTemplate` _createdtemplate))
        (bind _output_get (set `local.Local_currentCreatedTemplateActor` _parentactor))
        (set `local.Local_currentAssociateMeshes` _associativechildactor)
        (bind (_origin _extent) (`self.GetUnionBoundingBox` _output_get))
        (set `self.AccumulatedHeight` (+ (* (.z _extent) 1.98) (`self.AccumulatedHeight`)))
        (`self.GenerateAdditionalParts` (`local.Local_currentCreatedTemplateActor`) (`local.Local_currentAssociateMeshes`))))
    (:`then_1`
      (bind _output_get_2 (set `local.Local_middleFirescapeCount` (- (`self.TotalCount(IncludingStartAndEnd)`) (+ (select `bool` (`self.AddStartingPiece?`) :`true` 1) (select `bool` (`self.AddEndingPiece?`) :`true` 1)))))
      (for _index (range _output_get_2)
        (bind _output_get_3 (set `local.Local_currentStructureIndex` _index))
        (set `local.Local_isEvenIndex` (== (`KismetMathLibrary.FTrunc` (`KismetMathLibrary.FMod` (`KismetMathLibrary.Conv_IntToDouble` _output_get_3) 2.0)) 0))
        (bind _createdtemplate_2 (`self.CreateNewTemplate` (`self.FirescapeMiddleActor`)))
        (bind (_parentactor_2 _associativechildactor_2) (break `/Game/CyberTown/Blueprints/Procedural/Building/BlueprintStructures/S_CreatedTemplate` _createdtemplate_2))
        (bind _output_get_4 (set `local.Local_currentCreatedTemplateActor` _parentactor_2))
        (set `local.Local_currentAssociateMeshes` _associativechildactor_2)
        (`SceneComponent.K2_SetRelativeLocation` _output_get_4 (`KismetMathLibrary.MakeVector` 0.0 0.0 (`self.AccumulatedHeight`)) false false)
        (bind (_origin_2 _extent_2) (`self.GetUnionBoundingBox` (`local.Local_currentCreatedTemplateActor`)))
        (set `self.AccumulatedHeight` (+ (* (.z _extent_2) 1.996) (`self.AccumulatedHeight`)))
        (`self.GenerateAdditionalParts` (`local.Local_currentCreatedTemplateActor`) (`local.Local_currentAssociateMeshes`))))
    (:`then_2`
      (if (`self.AddEndingPiece?`)
        (bind _createdtemplate_3 (`self.CreateNewTemplate` (`self.FirescapeEndingActor`)))
        (bind (_parentactor_3 _associativechildactor_3) (break `/Game/CyberTown/Blueprints/Procedural/Building/BlueprintStructures/S_CreatedTemplate` _createdtemplate_3))
        (bind _output_get_5 (set `local.Local_currentCreatedTemplateActor` _parentactor_3))
        (set `local.Local_currentAssociateMeshes` _associativechildactor_3)
        (`SceneComponent.K2_SetRelativeLocation` _output_get_5 (`KismetMathLibrary.MakeVector` 0.0 0.0 (`self.AccumulatedHeight`)) false false)
        (set `local.Local_endFirescapePieceRotation` (select `bool` (`local.Local_isEvenIndex`) :`true` (struct :`Yaw` 180.0) :!type "Rotator Structure"))
        (`SceneComponent.K2_SetRelativeRotation` _local_currentcreatedtemplateactor (`KismetMathLibrary.ComposeRotators` (`SceneComponent.RelativeRotation` _local_currentcreatedtemplateactor) (`local.Local_endFirescapePieceRotation`)) false false)
        (bind (_origin_3 _extent_3) (`self.GetUnionBoundingBox` (`local.Local_currentCreatedTemplateActor`)))
        (set `self.AccumulatedHeight` (+ (* (.z _extent_3) 1.98) (`self.AccumulatedHeight`)))
        (`self.GenerateAdditionalParts` (`local.Local_currentCreatedTemplateActor`) (`local.Local_currentAssociateMeshes`))))))

(fn `ManageOptions`
  (bind _laddertransforms (`self.LadderTransforms`))
  (bind _associatemeshes (`self.AssociateMeshes`))
  (bind _associatemeshes_2 (`self.AssociateMeshes`))
  (bind _associatemeshes_3 (`self.AssociateMeshes`))
  (bind _value (`BlueprintMapLibrary.Map_Find` _associatemeshes "Ladder-3"))
  (bind _value_2 (`BlueprintMapLibrary.Map_Find` _associatemeshes_3 "Ladder-1"))
  (bind _value_3 (`BlueprintMapLibrary.Map_Find` _associatemeshes_2 "Ladder-2"))
  (`parent.ManageOptions`)
  (while (!= (`KismetArrayLibrary.Array_Length` (`self.LadderTransforms`)) (`self.LadderCount`))
    (if (< (`KismetArrayLibrary.Array_Length` (`self.LadderTransforms`)) (`self.LadderCount`))
      (`KismetArrayLibrary.Array_Add` (`self.LadderTransforms`))
      (else
        (`KismetArrayLibrary.Array_Remove` _laddertransforms (`KismetArrayLibrary.Array_LastIndex` _laddertransforms)))))
  ;[1 1 1] Associate Mesh Assigns.
  (`BlueprintMapLibrary.Map_Add` _associatemeshes_3 "Ladder-1" (make `/Game/CyberTown/Blueprints/Procedural/Building/BlueprintStructures/S_AdditionalPartArray` (and (`self.AddStartingLadder?`) (>= (`self.LadderCount`) 1)) (`.IgnoreSeed?_18_BDEB959A48F950CD154EA583AFFCC616` (break `/Game/CyberTown/Blueprints/Procedural/Building/BlueprintStructures/S_AdditionalPartArray` _value_2)) (`self.RandomnessSeed`) 0 (`.StaticMeshes_3_4713F08043DEA2AA411F85892B8F510C` (break `/Game/CyberTown/Blueprints/Procedural/Building/BlueprintStructures/S_AdditionalPartArray` _value_2)) (`|GetArrayItem` (`self.LadderTransforms`))))
  (`BlueprintMapLibrary.Map_Add` _associatemeshes_2 "Ladder-2" (make `/Game/CyberTown/Blueprints/Procedural/Building/BlueprintStructures/S_AdditionalPartArray` (and (`self.AddStartingLadder?`) (>= (`self.LadderCount`) 2)) (`.IgnoreSeed?_18_BDEB959A48F950CD154EA583AFFCC616` (break `/Game/CyberTown/Blueprints/Procedural/Building/BlueprintStructures/S_AdditionalPartArray` _value_3)) (`self.RandomnessSeed`) 0 (`.StaticMeshes_3_4713F08043DEA2AA411F85892B8F510C` (break `/Game/CyberTown/Blueprints/Procedural/Building/BlueprintStructures/S_AdditionalPartArray` _value_3)) (`|GetArrayItem` (`self.LadderTransforms`) 1)))
  (`BlueprintMapLibrary.Map_Add` _associatemeshes "Ladder-3" (make `/Game/CyberTown/Blueprints/Procedural/Building/BlueprintStructures/S_AdditionalPartArray` (and (`self.AddStartingLadder?`) (>= (`self.LadderCount`) 3)) (`.IgnoreSeed?_18_BDEB959A48F950CD154EA583AFFCC616` (break `/Game/CyberTown/Blueprints/Procedural/Building/BlueprintStructures/S_AdditionalPartArray` _value)) (`self.RandomnessSeed`) 0 (`.StaticMeshes_3_4713F08043DEA2AA411F85892B8F510C` (break `/Game/CyberTown/Blueprints/Procedural/Building/BlueprintStructures/S_AdditionalPartArray` _value)) (`|GetArrayItem` (`self.LadderTransforms`) 2))))

(fn `UserConstructionScript`
  (set `self.TotalCount(IncludingStartAndEnd)` (`KismetMathLibrary.Clamp` (`self.TotalCount(IncludingStartAndEnd)`) (+ (select `bool` (`self.AddStartingPiece?`) :`true` 1) (select `bool` (`self.AddEndingPiece?`) :`true` 1)) 50))
  (`parent.UserConstructionScript`))