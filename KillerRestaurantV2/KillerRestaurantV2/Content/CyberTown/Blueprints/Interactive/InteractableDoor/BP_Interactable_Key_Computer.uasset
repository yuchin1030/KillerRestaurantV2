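; Interactable key box computer that triggers a linked InteractableDoor when its Interact event fires.
; Construction creates a dynamic material and enables interaction if a door is assigned, while a timeline flashes the emissive color.
; Interacting messages the door, stops the flash and locks input until the door's transition-complete callback restores both.
; Overlap handlers only cast to Character, with player-side prompt and key logic left as unconnected setup examples.
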(event `/Game/CyberTown/Blueprints/Interactive/BP_Interactable.Interact`
  (bind _interactabledoor (`self.interactableDoor`))
  ;[1 1 1] Calls "Interact" interface on the InteractableDoor
  (if (and (`self.isInteractable`) (`self.notTransitioning`))
    (`/Engine/EditorBlueprintResources/StandardMacros.IsValid` _interactabledoor
      (:`Is Valid`
        (message `/Game/CyberTown/Blueprints/Interactive/BP_Interactable.Interact` _interactabledoor)
        (`TimelineComponent.Stop` (`self.FlashTimeline`))
        (`self.SetInteractable` (`self.notTransitioning`))
        (add `/Game/CyberTown/Blueprints/Interactive/InteractableDoor/BP_InteractableDoor.OnTransitionComplete` _interactabledoor (delegate `DoorTransitionComplete`))))))

(event `DoorTransitionComplete`
  ;[1 1 1] Calls "Interact" interface on the InteractableDoor
  (`self.SetInteractable` (`self.notTransitioning`) true)
  (`TimelineComponent.PlayFromStart` (`self.FlashTimeline`)))

(event `EnteredInteractArea[Implement this in your character BP]`
  (params (InteractActor :type "Actor Object Reference"))
  ;[0.1094 0.1094 0.1094] How to setup
  ;;[0 0.2582 0.5776] These events need to be implemented inside your player character BLUEPRINT. The references need to be created inside your blueprint (Interact Actor , Interact Widget)
)

(event `self.InteractCollision.OnComponentBeginOverlap`
  (params (OverlappedComponent :type "PrimitiveComponent Object Reference") (OtherActor :type "Actor Object Reference") (OtherComp :type "PrimitiveComponent Object Reference") (OtherBodyIndex :type Integer) (bFromSweep :type Boolean) (SweepResult :type "HitResult Structure (by ref)"))
  ;[0.1094 0.1094 0.1094] How to setup
  ;;[1 1 1] Notify Player Character to know it entered interactable area
  (if (`self.isInteractable`)
    (cast `Character` OtherActor)))

(event `ExitedInteractArea[Implement this in your character BP]`
  ;[0.1094 0.1094 0.1094] How to setup
  ;;[0 0.2582 0.5776] These events need to be implemented inside your player character BLUEPRINT. The references need to be created inside your blueprint (Interact Actor , Interact Widget)
)

(event `self.InteractCollision.OnComponentEndOverlap`
  (params (OverlappedComponent :type "PrimitiveComponent Object Reference") (OtherActor :type "Actor Object Reference") (OtherComp :type "PrimitiveComponent Object Reference") (OtherBodyIndex :type Integer))
  ;[0.1094 0.1094 0.1094] How to setup
  ;;[1 1 1] Notify Player Character to know it entered interactable area
  (if (`self.isInteractable`)
    (cast `Character` OtherActor)))

(event `OnPressE [Implement this in your character BP]`
  ;[0.1094 0.1094 0.1094] How to setup
  ;;[0 0.2582 0.5776] These events need to be implemented inside your player character BLUEPRINT. The references need to be created inside your blueprint (Interact Actor , Interact Widget)
)

(event `self.ReceiveBeginPlay`
  ;[1 1 1] Flashing Green Color Timeline
  (if (`self.isInteractable`)
    (bind (_direction _flashcolor) (`Timeline|FlashTimeline` :!via `PlayFromStart`)
      (:`Update`
        (`MaterialInstanceDynamic.SetVectorParameterValue` (`self.DynamicMaterial`) "Main_EmissiveColor" _flashcolor)))))

(fn `Initialize`
  (bind _sm_keybox_01a (`self.SM_KeyBox_01a`))
  (bind _returnvalue (`PrimitiveComponent.CreateDynamicMaterialInstance` _sm_keybox_01a 0 (`PrimitiveComponent.GetMaterial` _sm_keybox_01a 0) "None"))
  (set `self.DynamicMaterial` _returnvalue)
  (`/Engine/EditorBlueprintResources/StandardMacros.IsValid` (`self.interactableDoor`)
    (:`Is Valid`
      (bind _output_get (set `self.isInteractable` true))
      (`self.SetInteractable` (`self.isInteractable`) _output_get))))

(fn `SetInteractable`
  (params (b :type "Boolean (by ref)") (ref :type Boolean))
  (`|VariableSetRef` b ref)
  (if ref
    (`MaterialInstanceDynamic.SetVectorParameterValue` (`self.DynamicMaterial`) "Main_EmissiveColor" (`self.InteractableColor`))
    (else
      (`MaterialInstanceDynamic.SetVectorParameterValue` (`self.DynamicMaterial`) "Main_EmissiveColor" (`self.NotInteractableColor`)))))

(fn `UserConstructionScript`
  (`self.Initialize`))