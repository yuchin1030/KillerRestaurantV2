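; An interactable door Blueprint that slides its static mesh vertically between open and closed positions.
; Construction caches both world locations from the mesh's placed position, StartOpened state, bounds height and OpenedOffset, always along world up.
; Interact plays the open or close timeline, lerping location by its SpeedCurve without sweep.
; Interaction is ignored mid-transition; on finish the open state updates and CallOnTransitionComplete runs.
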(event `/Game/CyberTown/Blueprints/Interactive/BP_Interactable.Interact`
  (if (`self.isTransitioning`)
    _
    (elif (`self.isOpen`)
      (set `self.isTransitioning` true)
      (bind (_direction _speedcurve) (`Timeline|Close Timeline` :!via `PlayFromStart`)
        (:`Update`
          (`SceneComponent.K2_SetWorldLocation` (`self.StaticMeshComponent`) (`KismetMathLibrary.VLerp` (`self.cachedOpenLocation`) (`self.cachedCloseLocation`) _speedcurve) false false))
        (:`Finished`
          (set `self.isTransitioning` false)
          (set `self.isOpen` false)
          (`self.OnTransitionComplete`)))
      (else
        (set `self.isTransitioning` true)
        (bind (_direction_2 _speedcurve_2) (`Timeline|Open Timeline` :!via `PlayFromStart`)
          (:`Update`
            (`SceneComponent.K2_SetWorldLocation` (`self.StaticMeshComponent`) (`KismetMathLibrary.VLerp` (`self.cachedCloseLocation`) (`self.cachedOpenLocation`) _speedcurve_2) false false))
          (:`Finished`
            (set `self.isTransitioning` false)
            (set `self.isOpen` true)
            (`self.OnTransitionComplete`)))))))

(fn `Initialize`
  (bind _staticmeshcomponent (`self.StaticMeshComponent`))
  (bind _staticmeshcomponent_2 (`self.StaticMeshComponent`))
  (if (`self.startOpened`)
    (set `self.cachedOpenLocation` (`SceneComponent.K2_GetComponentLocation` _staticmeshcomponent_2))
    (set `self.cachedCloseLocation` (+ (* (`KismetMathLibrary.GetUpVector` (struct)) (- (* (.z (`.BoxExtent` (`KismetSystemLibrary.GetComponentBounds` _staticmeshcomponent_2))) -2.0) (`self.openedOffset`))) (`self.cachedOpenLocation`)))
    (set `self.isOpen` true)
    (else
      (set `self.cachedCloseLocation` (`SceneComponent.K2_GetComponentLocation` _staticmeshcomponent))
      (set `self.cachedOpenLocation` (+ (* (`KismetMathLibrary.GetUpVector` (struct)) (+ (* (.z (`.BoxExtent` (`KismetSystemLibrary.GetComponentBounds` _staticmeshcomponent))) 2.0) (`self.openedOffset`))) (`self.cachedCloseLocation`))))))

(fn `UserConstructionScript`
  (`self.Initialize`))