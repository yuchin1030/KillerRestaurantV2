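; Modular dungeon gateway door that acts as a portal, teleporting the third-person player character on contact.
; Entering its box trigger looks up PortalID in the PortalTeleport map and moves the character to the stored location, without sweep.
; A per-door boolean (NewVar) is set after the move, blocking further teleports from that door until the character's end-overlap clears it.
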(event `self.Box.OnComponentBeginOverlap`
  (params (OverlappedComponent :type "PrimitiveComponent Object Reference") (OtherActor :type "Actor Object Reference") (OtherComp :type "PrimitiveComponent Object Reference") (OtherBodyIndex :type Integer) (bFromSweep :type Boolean) (SweepResult :type "HitResult Structure (by ref)"))
  (bind (_value _returnvalue) (`BlueprintMapLibrary.Map_Find` (`self.PortalTeleport`) (`self.PortalID`)))
  (if (not (`self.NewVar`))
    (bind _asbp_third_person_character (cast `/Game/ThirdPerson/Blueprints/BP_ThirdPersonCharacter` OtherActor))
    (if _returnvalue
      (`self.K2_SetActorLocation` _asbp_third_person_character _value false false)
      (set `self.NewVar` true))))

(event `self.Box.OnComponentEndOverlap`
  (params (OverlappedComponent :type "PrimitiveComponent Object Reference") (OtherActor :type "Actor Object Reference") (OtherComp :type "PrimitiveComponent Object Reference") (OtherBodyIndex :type Integer))
  (if (`self.NewVar`)
    (cast `/Game/ThirdPerson/Blueprints/BP_ThirdPersonCharacter` OtherActor)
    (set `self.NewVar` false)))

(fn `UserConstructionScript`)